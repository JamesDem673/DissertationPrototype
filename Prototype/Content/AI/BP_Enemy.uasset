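; Enemy character that attacks with a sword montage, takes damage through a stats component and shows a health bar widget.
; Begin and end trace events toggle a looping timer that sphere-traces between two blade arrows for pawns, with debug drawing.
; A DoOnce with delayed reset throttles applied damage.
; Death disables movement, ragdolls the mesh, blocks further trace damage and destroys the widget.
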(event `self.ReceiveBeginPlay`
  ;[1 1 1] Init enemy health bar
  (bind _aswbp_enemy_health (cast `/Game/UI/WBP_EnemyHealth` (`WidgetComponent.GetWidget` (`self.Widget`))))
  (`/Game/Blueprints/BPC_Stats.SetHealthProgressBar` (`self.BPC_Stats`) (`/Game/UI/WBP_EnemyHealth.HealthBar` _aswbp_enemy_health)))

(event `self.ReceiveAnyDamage`
  (params (Damage :type "Float (single-precision)") (DamageType :type "DamageType Object Reference") (InstigatedBy :type "Controller Object Reference") (DamageCauser :type "Actor Object Reference"))
  ;[1 1 1] Updates health when injured
  (`/Game/Blueprints/BPC_Stats.Increase Value` (`self.BPC_Stats`) "NewEnumerator0" (* Damage -1.0)))

(event `/Game/Blueprints/BPI_Damage.EndSwordTrace`
  ;[1 1 1] Checks if the trace timer is active and stops it
  (if (`KismetSystemLibrary.K2_IsValidTimerHandle` (stale `/Game/Blueprints/BPI_Damage.BeginSwordTrace` _returnvalue))
    (`KismetSystemLibrary.K2_ClearAndInvalidateTimerHandle` (stale `/Game/Blueprints/BPI_Damage.BeginSwordTrace` _returnvalue))))

(event `/Game/Blueprints/BPI_Damage.BeginSwordTrace`
  ;[1 1 1] Creates a time that creates a trace for the sword every 0.1 seconds
  (bind _returnvalue (`KismetSystemLibrary.K2_SetTimerDelegate` (delegate `Damage Trace`) 0.01 true)))

(event `Damage Trace`
  ;[1 1 1] Sword trace for impact on enemies
  (if (not (`self.isDead`))
    (bind (_outhit _returnvalue) (`KismetSystemLibrary.SphereTraceSingleForObjects` :`Start` (`SceneComponent.K2_GetComponentLocation` (`self.Start Sword Trace Arrow`)) :`End` (`SceneComponent.K2_GetComponentLocation` (`self.End Sword Trace Arrow`)) :`Radius` 20.0 :`ObjectTypes` (`|MakeArray` "ObjectTypeQuery3" :!type "EObjectTypeQuery Enum") :`DrawDebugType` "ForDuration" :`DrawTime` 0.1))
    ;[1 1 1] Deals damage
    (if _returnvalue
      (`/Engine/EditorBlueprintResources/StandardMacros.DoOnce` false :!label _label
        (:`Completed`
          (`GameplayStatics.ApplyDamage` (`.HitActor` (`GameplayStatics.BreakHitResult` _outhit)) (`self.Sword Damage`))
          (`KismetSystemLibrary.Delay` 0.3)
          (goto _label :!via `Reset`))))))

(event `/Game/Blueprints/BPI_Damage.Death`
  ;[1 1 1] Handles enemy death
  (`CharacterMovementComponent.DisableMovement` (`self.CharacterMovement`))
  (`PrimitiveComponent.SetSimulatePhysics` (`self.Mesh`) true)
  (set `self.isDead` true)
  (`ActorComponent.K2_DestroyComponent` (`self.Widget`)))

(fn `Sword Attack`
  (returns (Duration :type "Float (double-precision)"))
  (bind _returnvalue (`self.PlayAnimMontage` "/Game/Characters/Animations/Combat/SwordAttackCombo_Montage.SwordAttackCombo_Montage"))
  (return _returnvalue))

(fn `UserConstructionScript`)