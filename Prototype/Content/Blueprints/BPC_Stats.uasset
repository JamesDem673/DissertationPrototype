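; BPC_Stats is a stats component that tracks its owner's health and handles death.
; IncreaseValue switches on the stat type, adds the amount to Health and clamps it between zero and MaxHealth.
; At zero health it fires Death, which sends DeathMessage to the owning actor.
; It also updates a health progress bar, supplied through SetHealthProgressBar, with the current health fraction.
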(event `Death`
  ;[1 1 1] Kills player
  (message `/Game/Blueprints/BPI_Damage.Death` (`self.GetOwner`)))

(event `SetHealthProgressBar`
  (params (HealthProgressBar :type "ProgressBar Object Reference"))
  (set `self.Health Progress Bar` HealthProgressBar))

(fn `Increase Value`
  (params (Stat :type "/Game/Blueprints/E_Stats Enum" :default "NewEnumerator0") (Value :type "Float (double-precision)"))
  ;[1 1 1] Increases value of specific stat by set amount
  (switch `/Game/Blueprints/E_Stats` Stat
    (:`NewEnumerator0`
      (set `self.Health` (`KismetMathLibrary.FClamp` (+ (`self.Health`) Value) 0.0 (`self.maxHealth`)))
      (`|ExecutionSequence`
        (:`then_0`
          ;[1 1 1] Checks if health is <= 0, then kills player if it is
          (if (<= (`self.Health`) 0.0)
            (`self.Death`)))
        (:`then_1`
          ;[1 1 1] Sets health bar once health updates
          (bind _health_progress_bar (`self.Health Progress Bar`)
            (:`then`
              (`ProgressBar.SetPercent` _health_progress_bar (/ (`self.Health`) (`self.maxHealth`))))
            (:`else`)))))))