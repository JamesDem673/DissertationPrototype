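; Melee enemy character with sword combo and big attack montages, a widget health bar, and backstab and knife-stagger reactions.
; Damage feeds BPCStats, which is linked to the health bar.
; A looping timer turns the enemy toward the player and sphere-traces between sword arrows with throttled damage, while a separate point trace handles slams.
; Death ragdolls the mesh, hides the bar, disables movement and collision, and notifies the player's BPCCombat.
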(event `self.ReceiveBeginPlay`
  ;[1 1 1] Init enemy health bar
  (bind _aswbp_enemy_health (cast `/Game/UI/WBP_EnemyHealth` (`WidgetComponent.GetWidget` (`self.Widget`))))
  (bind _healthbar (`/Game/UI/WBP_EnemyHealth.HealthBar` _aswbp_enemy_health))
  (`/Game/Blueprints/BPC_Stats.SetHealthProgressBar` (`self.BPC_Stats`) _healthbar)
  (set `self.Health Bar` _healthbar))

(event `self.ReceiveAnyDamage`
  (params (Damage :type "Float (single-precision)") (DamageType :type "DamageType Object Reference") (InstigatedBy :type "Controller Object Reference") (DamageCauser :type "Actor Object Reference"))
  ;[1 1 1] Updates health when injured
  (`/Game/Blueprints/BPC_Stats.Increase Value` (`self.BPC_Stats`) "NewEnumerator0" (* Damage -1.0)))

(event `/Game/Blueprints/BPI_Damage.EndSwordTrace`
  ;[1 1 1] Checks if the trace timer is active and stops it
  (if (`KismetSystemLibrary.K2_IsValidTimerHandle` (stale `/Game/Blueprints/BPI_Damage.BeginSwordTrace` _returnvalue))
    (`KismetSystemLibrary.K2_ClearAndInvalidateTimerHandle` (stale `/Game/Blueprints/BPI_Damage.BeginSwordTrace` _returnvalue))))

(event `/Game/Blueprints/BPI_Damage.BeginSwordTrace`
  ;[1 1 1] Creates a time that creates a trace for the sword every 0.1 seconds
  (bind _returnvalue (`KismetSystemLibrary.K2_SetTimerDelegate` (delegate `Damage Trace`) 0.01 true)))

(event `Damage Trace`
  ;[1 1 1] Sword trace for impact on enemies
  (if (not (`self.isDead`))
    (`self.K2_SetActorRotation` (`KismetMathLibrary.FindLookAtRotation` (`self.K2_GetActorLocation`) (`self.K2_GetActorLocation` (`GameplayStatics.GetPlayerPawn` 0))))
    (bind (_outhit _returnvalue) (`KismetSystemLibrary.SphereTraceSingleForObjects` :`Start` (`SceneComponent.K2_GetComponentLocation` (`self.Start Sword Trace Arrow`)) :`End` (`SceneComponent.K2_GetComponentLocation` (`self.End Sword Trace Arrow`)) :`Radius` 20.0 :`ObjectTypes` (`|MakeArray` "ObjectTypeQuery3" :!type "EObjectTypeQuery Enum") :`DrawDebugType` "ForDuration" :`DrawTime` 0.1))
    ;[1 1 1] Deals damage
    (if _returnvalue
      (`/Engine/EditorBlueprintResources/StandardMacros.DoOnce` false :!label _label
        (:`Completed`
          (`GameplayStatics.ApplyDamage` (`.HitActor` (`GameplayStatics.BreakHitResult` _outhit)) (`self.Sword Damage`))
          (`KismetSystemLibrary.Delay` 0.3)
          (goto _label :!via `Reset`))))))

(event `/Game/Blueprints/BPI_Damage.Death`
  ;[1 1 1] Handles enemy death
  (`CharacterMovementComponent.DisableMovement` (`self.CharacterMovement`))
  (`PrimitiveComponent.SetSimulatePhysics` (`self.Mesh`) true)
  (set `self.isDead` true)
  (bind _asbp_third_person_character (cast `/Game/ThirdPerson/Blueprints/BP_ThirdPersonCharacter` (`GameplayStatics.GetPlayerCharacter` 0)))
  (`/Game/Blueprints/BPC_Combat.EnemyDeath` (`/Game/ThirdPerson/Blueprints/BP_ThirdPersonCharacter.BPC_Combat` _asbp_third_person_character))
  (set `Widget.Visibility` "Hidden" (`self.Health Bar`))
  (`PrimitiveComponent.SetCollisionEnabled` (`self.CapsuleComponent`) "NoCollision"))

(event `/Game/Blueprints/BPI_Damage.PointDamageTrace`
  (bind _returnvalue (`SceneComponent.K2_GetComponentLocation` (`self.Point Trace Pos`)))
  ;[1 1 1] Slam check and damage
  (bind (_outhit _returnvalue_2) (`KismetSystemLibrary.SphereTraceSingleForObjects` :`Start` _returnvalue :`End` _returnvalue :`Radius` (`self.Radius`) :`ObjectTypes` (`|MakeArray` "ObjectTypeQuery3" :!type "EObjectTypeQuery Enum") :`DrawDebugType` "ForDuration" :`DrawTime` 1.0))
  (if _returnvalue_2
    (`GameplayStatics.ApplyDamage` (`.HitActor` (`GameplayStatics.BreakHitResult` _outhit)) 20.0)))

(event `/Game/Blueprints/BPI_Backstab.PerformBackstab`
  ;[1 1 1] Backstab death
  (`self.PlayAnimMontage` "/Game/Characters/Animations/Combat/A_Stealthkillvictem_Montage.A_Stealthkillvictem_Montage")
  (`KismetSystemLibrary.Delay` 1.5)
  (`GameplayStatics.ApplyDamage` self 999.0))

(event `HitByKnife`
  ;[1 1 1] Stagger
  (if (== (`self.GetCurrentMontage`) "/Game/Characters/Animations/Combat/SwordAttackCombo_Montage.SwordAttackCombo_Montage")
    (`self.StopAnimMontage` "/Game/Characters/Animations/Combat/SwordAttackCombo_Montage.SwordAttackCombo_Montage")))

(fn `Big Attack`
  (returns (Duration :type "Float (double-precision)"))
  (bind _returnvalue (`self.PlayAnimMontage` "/Game/Characters/Animations/Combat/BigAttack_Montage.BigAttack_Montage"))
  (return _returnvalue))

(fn `canBackstab`
  (returns (canBackstab :type Boolean))
  (return true))

(fn `Sword Attack`
  (returns (Duration :type "Float (double-precision)"))
  (bind _returnvalue (`self.PlayAnimMontage` "/Game/Characters/Animations/Combat/SwordAttackCombo_Montage.SwordAttackCombo_Montage"))
  (return _returnvalue))

(fn `UserConstructionScript`)