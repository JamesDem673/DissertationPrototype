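; Player combat component for BP_ThirdPersonCharacter, handling enemy lock-on, directional dodges, sword combos, backstabs and knife throws.
; Lock-on sphere-traces from the camera, attaches a marker actor and turns the controller toward the target every tick.
; Attack uses a forward trace and dot product to choose between a positioned backstab montage and a notify-gated combo.
; A looping timer sweeps the sword for hits, applying damage through a delayed-reset DoOnce.
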(event `self.ReceiveBeginPlay`
  ;[1 1 1] Sets player BP reference as a variable
  (bind _asbp_third_person_character (cast `/Game/ThirdPerson/Blueprints/BP_ThirdPersonCharacter` (`self.GetOwner`)))
  (set `self.PlayerBP` _asbp_third_person_character))

(event `EnemyDeath`
  (bind _charactermovement (`Character.CharacterMovement` (`self.PlayerBP`)))
  ;[1 1 1] Disables lock on when enemy dies
  (`self.Target Lock Actor`
    (:`then`
      ;[1 1 1] Unlocks player from actor focus and removes target lock widget
      (set `self.Target Lock Actor` null :!label _label)
      (set `CharacterMovementComponent.bOrientRotationToMovement` true _charactermovement)
      (set `CharacterMovementComponent.bUseControllerDesiredRotation` false _charactermovement)
      (`Actor.K2_DestroyActor` (`self.Target Lock Widget`)))
    (:`else`)))

(event `EnhancedInput|/Game/ThirdPerson/Input/Actions/IA_Lock`
  (params (ActionValue :type Boolean) (ElapsedSeconds :type "Float (double-precision)") (TriggeredSeconds :type "Float (double-precision)") (InputAction :type "InputAction Object Reference" :default "/Game/ThirdPerson/Input/Actions/IA_Lock.IA_Lock"))
  (bind _returnvalue (`Actor.GetTransform` (`self.Target Lock Actor`)))
  (bind _transformcomponent (`PlayerCameraManager.TransformComponent` (`GameplayStatics.GetPlayerCameraManager` 0)))
  (bind _charactermovement (`Character.CharacterMovement` (`self.PlayerBP`)))
  (bind (_returnvalue_x _returnvalue_y _returnvalue_z) (`KismetMathLibrary.BreakVector` (`SceneComponent.K2_GetComponentLocation` _transformcomponent)))
  (bind _returnvalue_2 (`KismetMathLibrary.MakeVector` _returnvalue_x _returnvalue_y (+ _returnvalue_z 20.0)))
  ;[1 1 1] Checks if player is locked on already
  (:`Started`
    (`self.Target Lock Actor`
      (:`then`
        (goto _label))
      (:`else`
        ;[1 1 1] Trace to find actor to lock on to
        (bind (_outhit _returnvalue_3) (`KismetSystemLibrary.SphereTraceSingleForObjects` :`Start` _returnvalue_2 :`End` (+ _returnvalue_2 (* (`KismetMathLibrary.GetForwardVector` (`SceneComponent.K2_GetComponentRotation` _transformcomponent)) 1000.0)) :`Radius` 150.0 :`ObjectTypes` (`|MakeArray` "ObjectTypeQuery3" :!type "EObjectTypeQuery Enum") :`DrawDebugType` "ForDuration" :`DrawTime` 2.0))
        ;[1 1 1] Sets lock target and camera movement to match
        (if _returnvalue_3
          (bind (_bblockinghit _binitialoverlap _time _distance _location _impactpoint _normal _impactnormal _physmat _hitactor) (`GameplayStatics.BreakHitResult` _outhit))
          (bind _asbp_enemy (cast `/Game/Blueprints/TutorialBasedBps/AI/BP_Enemy` _hitactor))
          (if (not (`/Game/Blueprints/TutorialBasedBps/AI/BP_Enemy.isDead` _asbp_enemy))
            (set `self.Target Lock Actor` _hitactor)
            (set `CharacterMovementComponent.bOrientRotationToMovement` false _charactermovement)
            (set `CharacterMovementComponent.bUseControllerDesiredRotation` true _charactermovement)
            ;[1 1 1] Creates wdiget to show lock on and connects it to target actor
            (bind _returnvalue_4 (`|SpawnActorFromClass` "/Game/Blueprints/TutorialBasedBps/BP_TargetLockWidget.BP_TargetLockWidget_C" (`KismetMathLibrary.MakeTransform` (`KismetMathLibrary.MakeVector` (.x (.location _returnvalue)) (.y (.location _returnvalue)) (+ (.z (.location _returnvalue)) 20.0)) (.rotation _returnvalue)) "AlwaysSpawn" "MultiplyWithRoot" null null))
            (bind _output_get (set `self.Target Lock Widget` _returnvalue_4))
            (`Actor.K2_AttachToActor` _output_get (`self.Target Lock Actor`) "None" "SnapToTarget" "SnapToTarget" "SnapToTarget" true)))))))

(event `self.ReceiveTick`
  (params (DeltaSeconds :type "Float (single-precision)"))
  (bind (_returnvalue_roll _returnvalue_pitch _returnvalue_yaw) (`KismetMathLibrary.BreakRotator` (`KismetMathLibrary.FindLookAtRotation` (`Actor.K2_GetActorLocation` (`self.PlayerBP`)) (`Actor.K2_GetActorLocation` (`self.Target Lock Actor`)))))
  ;[1 1 1] Each tick updates player rotation (if locked on) to deal with movement
  (`self.Target Lock Actor`
    (:`then`
      (`Controller.SetControlRotation` (`Pawn.GetController` (`self.PlayerBP`)) (`KismetMathLibrary.MakeRotator` _returnvalue_roll (+ _returnvalue_pitch -20.0) _returnvalue_yaw)))
    (:`else`)))

(event `MoveToTarget`
  (params (Target :type "Actor Object Reference"))
  ;[1 1 1] When backstab is allowed, sets the player to behind the target actor
  (bind _asbp_third_person_character (cast `/Game/ThirdPerson/Blueprints/BP_ThirdPersonCharacter` (`self.GetOwner`)))
  (`KismetSystemLibrary.MoveComponentTo` (`Character.CapsuleComponent` _asbp_third_person_character) (- (`Actor.K2_GetActorLocation` Target) (* (`Actor.GetActorForwardVector` Target) 70.0)) (`Actor.K2_GetActorRotation` Target)))

(event `End Damage Trace`
  ;[1 1 1] Checks if the trace timer is active and stops it
  (if (`KismetSystemLibrary.K2_IsValidTimerHandle` (stale `Begin Damage Trace` _returnvalue))
    (`KismetSystemLibrary.K2_ClearAndInvalidateTimerHandle` (stale `Begin Damage Trace` _returnvalue))))

(event `Begin Damage Trace`
  ;[1 1 1] Creates a time that creates a trace for the sword every 0.1 seconds
  (bind _returnvalue (`KismetSystemLibrary.K2_SetTimerDelegate` (delegate `Damage Trace`) 0.01 true)))

(event `Damage Trace`
  (bind _playerbp (`self.PlayerBP`))
  ;[1 1 1] Sword trace for impact on enemies
  (bind (_outhit _returnvalue) (`KismetSystemLibrary.SphereTraceSingleForObjects` :`Start` (`SceneComponent.K2_GetComponentLocation` (`/Game/ThirdPerson/Blueprints/BP_ThirdPersonCharacter.Start Sword Trace Pos` _playerbp)) :`End` (`SceneComponent.K2_GetComponentLocation` (`/Game/ThirdPerson/Blueprints/BP_ThirdPersonCharacter.End  Sword Trace Pos` _playerbp)) :`Radius` 20.0 :`ObjectTypes` (`|MakeArray` "ObjectTypeQuery3" :!type "EObjectTypeQuery Enum") :`DrawDebugType` "ForDuration" :`DrawTime` 0.1))
  ;[1 1 1] Deals damage
  (if _returnvalue
    (`/Engine/EditorBlueprintResources/StandardMacros.DoOnce` false :!label _label_2
      (:`Completed`
        (`GameplayStatics.ApplyDamage` (`.HitActor` (`GameplayStatics.BreakHitResult` _outhit)) (`self.Sword Damage`))
        (`KismetSystemLibrary.Delay` 0.3)
        (goto _label_2 :!via `Reset`)))))

(event `EnhancedInput|/Game/ThirdPerson/Input/Actions/IA_Dodge`
  (params (ActionValue :type Boolean) (ElapsedSeconds :type "Float (double-precision)") (TriggeredSeconds :type "Float (double-precision)") (InputAction :type "InputAction Object Reference" :default "/Game/ThirdPerson/Input/Actions/IA_Dodge.IA_Dodge"))
  ;[1 1 1] Checks if player can dodge and lets them if yes
  (:`Started`
    (if (not (`self.IsDodging`))
      (set `self.IsDodging` true)
      (`|ExecutionSequence`
        (:`then_0`
          ;[1 1 1] Check if player is locked onto an enemy
          (if (`CharacterMovementComponent.bUseControllerDesiredRotation` (`Character.CharacterMovement` (`self.PlayerBP`)))
            ;[1 1 1] Sets player to roll in desired direction
            (switch `string` (`KismetTextLibrary.Conv_TextToString` (`KismetInputLibrary.Key_GetDisplayName` (`/Game/ThirdPerson/Blueprints/BP_ThirdPersonCharacter.Direction Key` (`self.PlayerBP`))))
              (:`Default`
                (set `self.MovementDirection` "NewEnumerator2" :!label _label_3))
              (:`W`
                (set `self.MovementDirection` "NewEnumerator0"))
              (:`A`
                (set `self.MovementDirection` "NewEnumerator1"))
              (:`S`
                (set `self.MovementDirection` "NewEnumerator3"))
              (:`D`
                (goto _label_3)))
            (else
              (set `self.MovementDirection` "NewEnumerator0"))))
        (:`then_1`
          ;[1 1 1] Plays roll animation
          (`|PlayMontage` (`Character.Mesh` (`self.PlayerBP`)) (select `/Game/Blueprints/TutorialBasedBps/E_MovementDirection` (`self.MovementDirection`) :`NewEnumerator0` "/Game/Characters/Animations/Combat/Dodge/Dodge_F_Montage.Dodge_F_Montage" :`NewEnumerator1` "/Game/Characters/Animations/Combat/Dodge/Dodge_L_Montage.Dodge_L_Montage" :`NewEnumerator2` "/Game/Characters/Animations/Combat/Dodge/Dodge_R_Montage.Dodge_R_Montage" :`NewEnumerator3` "/Game/Characters/Animations/Combat/Dodge/Dodge_B_Montage.Dodge_B_Montage" :!type "AnimMontage Object Reference")
            (:`OnCompleted`
              _)
            (:`OnInterrupted`
              _))
          (set `self.IsDodging` false))))))

(event `EnhancedInput|/Game/ThirdPerson/Input/Actions/IA_Attack`
  (params (ActionValue :type Boolean) (ElapsedSeconds :type "Float (double-precision)") (TriggeredSeconds :type "Float (double-precision)") (InputAction :type "InputAction Object Reference" :default "/Game/ThirdPerson/Input/Actions/IA_Attack.IA_Attack"))
  (bind _returnvalue (`self.GetOwner`))
  (bind _returnvalue_2 (`Actor.K2_GetActorLocation` _returnvalue))
  ;[1 1 1] Sphere trace in front of actor swinging
  (:`Started`
    (bind (_outhit _returnvalue_3) (`KismetSystemLibrary.SphereTraceSingleForObjects` _returnvalue_2 (+ _returnvalue_2 (* (`KismetMathLibrary.GetForwardVector` (`Actor.K2_GetActorRotation` _returnvalue)) 100.0)) 50.0 (`|MakeArray` "ObjectTypeQuery3" :!type "EObjectTypeQuery Enum")))
    ;[1 1 1] Checks if backstab or normal attack
    (if _returnvalue_3
      (bind (_bblockinghit _binitialoverlap _time _distance _location _impactpoint _normal _impactnormal _physmat _hitactor) (`GameplayStatics.BreakHitResult` _outhit))
      (if (< (`KismetMathLibrary.Dot_VectorVector` (`Actor.GetActorForwardVector` _hitactor) (`KismetMathLibrary.Normal` (- (`Actor.K2_GetActorLocation` (`self.GetOwner`)) (`Actor.K2_GetActorLocation` _hitactor)))) 0.0)
        ;[1 1 1] Performs backstab
        (if (not (`self.IsAttacking`))
          (set `self.IsAttacking` true)
          (`self.PerformBackstab`)
          (`KismetSystemLibrary.Delay` 1.0)
          (set `self.IsAttacking` false))
        (else
          ;[1 1 1] Plays combat animations after checking if not already
          (if (not (`self.IsAttacking`)) :!label _label_4
            (set `self.IsAttacking` true)
            (`|PlayMontage` (`Character.Mesh` (`self.PlayerBP`)) "/Game/Characters/Animations/Combat/SwordAttackCombo_Montage.SwordAttackCombo_Montage"
              (:`OnCompleted`
                ;[1 1 1] Allows for combo hits or cuts the animation if full 3 attacks aren't called
                (set `self.IsAttacking` false :!label _label_5)
                (set `self.IsCombo` false))
              (:`OnInterrupted`
                (goto _label_5))
              (:`OnNotifyBegin`
                (if (and (`self.IsAttacking`) (`self.IsCombo`))
                  (set `self.IsCombo` false)
                  (else
                    (`AnimInstance.Montage_Stop` (`SkeletalMeshComponent.GetAnimInstance` (`Character.Mesh` (`self.PlayerBP`))) 0.2 "/Game/Characters/Animations/Combat/SwordAttackCombo_Montage.SwordAttackCombo_Montage")))))
            (else
              (set `self.IsCombo` true)))))
      (else
        (goto _label_4)))))

(event `EnhancedInput|/Game/ThirdPerson/Input/Actions/IA_KnifeThrow`
  (params (ActionValue :type Boolean) (ElapsedSeconds :type "Float (double-precision)") (TriggeredSeconds :type "Float (double-precision)") (InputAction :type "InputAction Object Reference" :default "/Game/ThirdPerson/Input/Actions/IA_KnifeThrow.IA_KnifeThrow"))
  (:`Started`
    (bind _asbp_third_person_character (cast `/Game/ThirdPerson/Blueprints/BP_ThirdPersonCharacter` (`self.GetOwner`)))
    (bind _spawntransform (`/Game/ThirdPerson/Blueprints/BP_ThirdPersonCharacter.KnifeSpawn` _asbp_third_person_character))
    (`|SpawnActorFromClass` "/Game/Blueprints/BP_ThrowingKnife.BP_ThrowingKnife_C" _spawntransform "Undefined" "MultiplyWithRoot" null null)))

(fn `PerformBackstab`
  (locals (L_HitActor :type "Actor Object Reference"))
  (bind _returnvalue (`self.GetOwner`))
  (bind _returnvalue_2 (`Actor.K2_GetActorLocation` _returnvalue))
  (bind (_outhit _returnvalue_3) (`KismetSystemLibrary.SphereTraceSingleForObjects` :`Start` _returnvalue_2 :`End` (+ _returnvalue_2 (* (`KismetMathLibrary.GetForwardVector` (`Actor.K2_GetActorRotation` _returnvalue)) 100.0)) :`Radius` 20.0 :`ObjectTypes` (`|MakeArray` "ObjectTypeQuery3" :!type "EObjectTypeQuery Enum") :`DrawDebugType` "ForDuration"))
  (if _returnvalue_3
    (bind _output_get (set `local.L_HitActor` (`.HitActor` (`GameplayStatics.BreakHitResult` _outhit))))
    (bind _canbackstab (message `/Game/Blueprints/TutorialBasedBps/BPI_Backstab.canBackstab` _output_get))
    (if _canbackstab
      (if (not (`AnimInstance.IsAnyMontagePlaying` (`SkeletalMeshComponent.GetAnimInstance` (`Character.Mesh` (`self.PlayerBP`)))))
        (`self.MoveToTarget` (`local.L_HitActor`))
        (`Character.PlayAnimMontage` (`self.PlayerBP`) "/Game/Characters/Animations/Combat/A_StealthKillplayer_Montage.A_StealthKillplayer_Montage" 1.0 "None")
        (message `/Game/Blueprints/TutorialBasedBps/BPI_Backstab.PerformBackstab` (`local.L_HitActor`))))))